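; VNTrigger is an interactable trigger that sends the player into the VNEvent01 level.
; Overlapping its capsule adds an InteractWidget to the viewport, and leaving the capsule removes it.
; Interact fires run2, which clears all widgets, shows a Fadeout widget for a one-second delay, removes it and opens the hard-coded level by name.
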(event OnComponentBeginOverlap(Capsule)
  (params (OverlappedComponent :type Primitive%20Component%20Object%20Reference) (OtherActor :type Actor%20Object%20Reference) (OtherComp :type Primitive%20Component%20Object%20Reference) (OtherBodyIndex :type Integer) (bFromSweep :type Boolean) (SweepResult :type Hit%20Result%20Structure%20%28by%20ref%29))
  (bind _returnvalue (UserInterface|CreateWidget "/Game/UI/Blueprints/InteractWidget.InteractWidget_C"))
  (UserInterface|Viewport|AddtoViewport _returnvalue 0))

(event OnComponentEndOverlap(Capsule)
  (params (OverlappedComponent :type Primitive%20Component%20Object%20Reference) (OtherActor :type Actor%20Object%20Reference) (OtherComp :type Primitive%20Component%20Object%20Reference) (OtherBodyIndex :type Integer))
  (bind _foundwidgets (Widget|GetAllWidgetsOfClass "/Game/UI/Blueprints/InteractWidget.InteractWidget_C" true))
  (Widget|RemovefromParent _foundwidgets))

(event Custom|run2
  (Viewport|RemoveAllWidgets)
  (bind _returnvalue (UserInterface|CreateWidget "/Game/UI/VisualNovel/Blueprints/Fadeout.Fadeout_C"))
  (UserInterface|Viewport|AddtoViewport _returnvalue 0)
  (Utilities|FlowControl|Delay 1.0)
  (bind _foundwidgets (Widget|GetAllWidgetsOfClass "/Game/UI/VisualNovel/Blueprints/Fadeout.Fadeout_C" true))
  (Widget|RemovefromParent _foundwidgets)
  (Game|OpenLevel(byName) "VNEvent01"))

(fn ConstructionScript)

(fn Interact
  (CallFunction|Run2)
  (return false))