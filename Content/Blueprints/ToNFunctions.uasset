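; ToNFunctions is a helper function collection for restoring saved music volume and stepping float values.
; MusicVolumeCheck loads the SliderChange save, if present, and applies its slider position to the music sound class through a sound mix override.
; FakeLerp is built as a speed-times-delta-time step clamped at the target, but both direction multipliers are zero, so it returns the current value unchanged.
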(fn MusicVolumeCheck
  (SaveGame|DoesSaveGameExist "SliderChange")
  (if true
    (bind _returnvalue (SaveGame|LoadGamefromSlot "SliderChange"))
    (bind _asvolume_change (Utilities|Casting|CastToVolumeChange _returnvalue))
    (bind _output_get (Variables|/Game/Blueprints/VolumeChange.VolumeChange_C|SetSliderPosition _asvolume_change (Variables|/Game/Blueprints/VolumeChange.VolumeChange_C|GetSliderPosition _asvolume_change)))
    (Audio|SetSoundMixClassOverride 0 "/Game/UI/Music/NewSoundMix.NewSoundMix" "/Game/UI/Music/MusicClass.MusicClass" _output_get 1.0 0.0 true)
    (return)))

(fn FakeLerp
  (params (Current%20Value :type Float%20%28single-precision%29) (Target%20Value :type Float%20%28single-precision%29) (Delta%20Time :type Float%20%28single-precision%29) (Speed :type Float%20%28single-precision%29))
  (bind _returnvalue (< Current%20Value Target%20Value))
  (bind _returnvalue_2 (Math|Float|SelectFloat 0.0 0.0 _returnvalue))
  (bind _returnvalue_3 (* Delta%20Time Speed _returnvalue_2))
  (bind _returnvalue_4 (+ _returnvalue_3 Current%20Value))
  (return (Math|Float|SelectFloat (Math|Float|Min(Float) _returnvalue_4 Target%20Value) (Math|Float|Max(Float) _returnvalue_4 Target%20Value) _returnvalue)))