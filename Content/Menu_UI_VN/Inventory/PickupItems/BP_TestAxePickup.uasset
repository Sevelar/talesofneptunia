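; Test axe pickup actor that adds an axe to the player's inventory when its Box trigger is overlapped.
; On overlap it finds the first top-level Inventory widget and checks its eight slot values in order through nested branches.
; The first empty slot receives the axe item ID and the actor destroys itself; if all slots are full, it stays in place.
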(event OnComponentBeginOverlap(Box)
  (params (OverlappedComponent :type Primitive%20Component%20Object%20Reference) (OtherActor :type Actor%20Object%20Reference) (OtherComp :type Primitive%20Component%20Object%20Reference) (OtherBodyIndex :type Integer) (bFromSweep :type Boolean) (SweepResult :type Hit%20Result%20Structure%20%28by%20ref%29))
  (bind _foundwidgets (Widget|GetAllWidgetsOfClass "/Game/Menu_UI_VN/Inventory/Inventory.Inventory_C" true))
  (bind _asinventory (Utilities|Casting|CastToInventory (Utilities|Array|Get(acopy) _foundwidgets)))
  (if (== (Variables|/Game/Menu_UI_VN/Inventory/Inventory.Inventory_C|GetInvSlotValue1 _asinventory) 0)
    (Variables|/Game/Menu_UI_VN/Inventory/Inventory.Inventory_C|SetInvSlotValue1 _asinventory 5)
    (Actor|DestroyActor :!label _label)
    (elif (== (Variables|/Game/Menu_UI_VN/Inventory/Inventory.Inventory_C|GetInvSlotValue2 _asinventory) 0)
      (Variables|/Game/Menu_UI_VN/Inventory/Inventory.Inventory_C|SetInvSlotValue2 _asinventory 5)
      (goto _label)
      (elif (== (Variables|/Game/Menu_UI_VN/Inventory/Inventory.Inventory_C|GetInvSlotValue3 _asinventory) 0)
        (Variables|/Game/Menu_UI_VN/Inventory/Inventory.Inventory_C|SetInvSlotValue3 _asinventory 5)
        (goto _label)
        (elif (== (Variables|/Game/Menu_UI_VN/Inventory/Inventory.Inventory_C|GetInvSlotValue4 _asinventory) 0)
          (Variables|/Game/Menu_UI_VN/Inventory/Inventory.Inventory_C|SetInvSlotValue4 _asinventory 5)
          (goto _label)
          (elif (== (Variables|/Game/Menu_UI_VN/Inventory/Inventory.Inventory_C|GetInvSlotValue5 _asinventory) 0)
            (Variables|/Game/Menu_UI_VN/Inventory/Inventory.Inventory_C|SetInvSlotValue5 _asinventory 5)
            (goto _label)
            (elif (== (Variables|/Game/Menu_UI_VN/Inventory/Inventory.Inventory_C|GetInvSlotValue6 _asinventory) 0)
              (Variables|/Game/Menu_UI_VN/Inventory/Inventory.Inventory_C|SetInvSlotValue6 _asinventory 5)
              (goto _label)
              (elif (== (Variables|/Game/Menu_UI_VN/Inventory/Inventory.Inventory_C|GetInvSlotValue7 _asinventory) 0)
                (Variables|/Game/Menu_UI_VN/Inventory/Inventory.Inventory_C|SetInvSlotValue7 _asinventory 5)
                (goto _label)
                (elif (== (Variables|/Game/Menu_UI_VN/Inventory/Inventory.Inventory_C|GetInvSlotValue8 _asinventory) 0)
                  (Variables|/Game/Menu_UI_VN/Inventory/Inventory.Inventory_C|SetInvSlotValue8 _asinventory 5)
                  (goto _label))))))))))

(event EventBeginPlay)

(event Collision|EventActorBeginOverlap
  (params (OtherActor :type Actor%20Object%20Reference)))

(event EventTick
  (params (DeltaSeconds :type Float%20%28single-precision%29)))

(fn ConstructionScript)